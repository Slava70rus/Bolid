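; BP_Bolid is a drivable vehicle that passes player input to its VehicleMovement component.
; The MoveForward and MoveRight axes drive throttle and steering directly.
; The Handbrake action engages the handbrake and activates the PSDraw and PSDraw1 effects while held, then switches both off on release.
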(event Input|ActionEvents|InputActionHandbrake
  (params (Key :type Key%20Structure :default "None"))
  (bind _vehiclemovement (Variables|Default|GetVehicleMovement))
  (bind _ps_draw_ (Variables|Default|GetPS_Draw_))
  ;[1 1 1] Comment
  (:Pressed
    (Class|WheeledVehicleMovementComponent|SetHandbrakeInput _vehiclemovement true)
    (Components|Activation|SetActive _ps_draw_ true false))
  (:Released
    (Class|WheeledVehicleMovementComponent|SetHandbrakeInput _vehiclemovement false)
    (Components|Activation|SetActive _ps_draw_ false false)))

(event Input|AxisEvents|InputAxisMoveForward
  (params (AxisValue :type Float%20%28single-precision%29))
  ;[1 1 1] Throttle and Steering
  (Class|WheeledVehicleMovementComponent|SetThrottleInput (Variables|Default|GetVehicleMovement) AxisValue))

(event Input|AxisEvents|InputAxisMoveRight
  (params (AxisValue :type Float%20%28single-precision%29))
  ;[1 1 1] Throttle and Steering
  (Class|WheeledVehicleMovementComponent|SetSteeringInput (Variables|Default|GetVehicleMovement) AxisValue))

(fn ConstructionScript)